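; Player controller Blueprint that creates the main HUD and handles manual world saving.
; On BeginPlay, the local controller adds the HUD to the viewport, sets game-only input and binds to the game mode's save-written event.
; Pressing L asks the game mode to write the save, and the bound event shows a "Game Saved" notification on the HUD.
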(event `self.ReceiveBeginPlay`
  (if (`self.IsLocalController`)
    (bind _returnvalue (`|CreateWidget` "/Game/TomLoomanCppProject/UI/Main_HUD.Main_HUD_C" self))
    (bind _output_get (set `self.HUD_Widget` _returnvalue))
    (`UserWidget.AddToViewport` _output_get 0)
    (`WidgetBlueprintLibrary.SetInputMode_GameOnly` self)
    (add `SGameModeBase.OnSaveGameWritten` (cast `SGameModeBase` (`GameplayStatics.GetGameMode`) :!pure true) (delegate `OnSaveGameWritten_Event`))))

(event `Key|L`
  (params (Key :type "Key Structure"))
  (:`Pressed`
    (bind _assgame_mode_base (cast `SGameModeBase` (`GameplayStatics.GetGameMode`)))
    (`SGameModeBase.WriteSaveGame` _assgame_mode_base)
    (`KismetSystemLibrary.PrintString` "WORLD SAVED!")))

(event `OnSaveGameWritten_Event`
  (params (SaveObject :type "SSaveGame Object Reference"))
  (`/Game/TomLoomanCppProject/UI/NotificationContainer_Widget.AddNotification` (`/Game/TomLoomanCppProject/UI/Main_HUD.NotificationContainer_Widget` (`self.HUD_Widget`)) "Game Saved" 4.0))

(fn `UserConstructionScript`)