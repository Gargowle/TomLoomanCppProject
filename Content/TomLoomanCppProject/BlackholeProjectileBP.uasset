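; Black hole projectile that destroys physics-simulating actors it overlaps.
; On spawn, its sphere component ignores the instigator when moving, so it does not self-destruct in the character's hand, and a timer destroys the projectile after a few seconds.
; On overlap, it destroys the other actor only if that actor's root component is simulating physics.
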(event `self.ReceiveBeginPlay`
  ;[1 1 1] Prevent direct self destruction in hand of character
  (`PrimitiveComponent.IgnoreActorWhenMoving` (`self.SphereComp`) (`self.GetInstigator`) true)
  (`KismetSystemLibrary.K2_SetTimerDelegate` (delegate `SelfDestruction_Event`) 5.0))

(event `SelfDestruction_Event`
  (`self.K2_DestroyActor`))

(event `self.ReceiveActorBeginOverlap`
  (params (OtherActor :type "Actor Object Reference"))
  (if (`SceneComponent.IsAnySimulatingPhysics` (`Actor.RootComponent` OtherActor))
    (`self.K2_DestroyActor` OtherActor)))

(fn `UserConstructionScript`)